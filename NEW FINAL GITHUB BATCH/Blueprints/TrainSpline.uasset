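; TrainSpline is a spline actor that spawns PC_Train pawns at the start of its spline, aligned to the spline's rotation.
; It spawns one train a second after play begins, while a Delay on Tick repeats the spawn at random intervals of several seconds.
; The construction script stores its index among all TrainSpline actors, which each spawned train receives as SplineIndex to link it to this spline.
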(event EventBeginPlay
  ;[1 1 1] On play, wait a moment, then spawn a train
  (Utilities|FlowControl|Delay 1.0)
  (CallFunction|SpawnTrain))

(event EventTick
  (params (DeltaSeconds :type Float%20%28single-precision%29))
  ;[1 1 1] Spawn a train at a randomly chosen interval
  (Utilities|FlowControl|Delay (Math|Random|RandomFloatinRange 5.0 15.0))
  (CallFunction|SpawnTrain))

(fn ConstructionScript
  ;[1 1 1] Get all splines and identify each entity as itself
  (bind _outactors (Actor|GetAllActorsOfClass "TrainSpline_C"))
  (Variables|Default|SetTrainSpline (Utilities|Array|FindItem _outactors self)))

(fn SpawnTrain
  (bind _spline (Variables|Default|GetSpline))
  ;[1 1 1] Get starting point of spline, then spawn a train at that point, give the train and spline a shared index
  (bind _returnvalue (AI|SpawnAIFromClass "/Game/Blueprints/PC_Train.PC_Train_C" 0 (Spline|GetLocationatDistanceAlongSpline _spline 0.0 "World") (Spline|GetRotationatDistanceAlongSpline _spline 0.0 "World") false))
  (bind _aspc_train (Utilities|Casting|CastToPC_Train _returnvalue))
  (Variables|/Game/Blueprints/PC_Train.PC_Train_C|SetSplineIndex _aspc_train (Variables|Default|GetTrainSpline)))