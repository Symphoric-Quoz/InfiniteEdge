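; PlayerCharacter is a player-controlled Character with directional movement and a zoomable orthographic camera.
; MoveForward and MoveRight axis inputs feed AddMovementInput along forward and right vectors built from control rotation yaw alone.
; Mouse wheel up and down shrink or widen the Camera's OrthoWidth in fixed, clamped steps to zoom in and out.
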(event Input|AxisEvents|InputAxisMoveRight
  (params (AxisValue :type Float%20%28single-precision%29))
  (Pawn|Input|AddMovementInput (Math|Vector|GetRightVector (Math|Rotator|MakeRotator 0.0 0.0 (.Yaw (Math|Rotator|BreakRotator (Pawn|GetControlRotation :!class /Script/Engine.Pawn))))) AxisValue false))

(event Input|AxisEvents|InputAxisMoveForward
  (params (AxisValue :type Float%20%28single-precision%29))
  (Pawn|Input|AddMovementInput (Math|Vector|GetForwardVector (Math|Rotator|MakeRotator 0.0 0.0 (.Yaw (Math|Rotator|BreakRotator (Pawn|GetControlRotation :!class /Script/Engine.Pawn))))) AxisValue false))

(event Input|MouseEvents|MouseWheelDown
  (params (Key :type Key%20Structure :default "AnyKey"))
  (:Pressed
    (Variables|/Script/Engine.CameraComponent|SetOrthoWidth (Variables|Default|GetCamera) (Math|Float|Clamp(Float) (+ (Variables|/Script/Engine.CameraComponent|GetOrthoWidth (Variables|Default|GetCamera)) 5e+01) 5e+02 2e+03))))

(event Input|MouseEvents|MouseWheelUp
  (params (Key :type Key%20Structure :default "AnyKey"))
  (:Pressed
    (Variables|/Script/Engine.CameraComponent|SetOrthoWidth (Variables|Default|GetCamera) (Math|Float|Clamp(Float) (- (Variables|/Script/Engine.CameraComponent|GetOrthoWidth (Variables|Default|GetCamera)) 5e+01) 5e+02 2e+03))))

(fn ConstructionScript)