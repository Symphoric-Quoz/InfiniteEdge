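; PedestrianSpline is a spline-based Blueprint that spawns a pedestrian at the start of its path.
; A short delay after BeginPlay, it calls SpawnPedestrian once and prints a debug string.
; SpawnPedestrian spawns a PC_Pedestrian AI at the spline's first point, matching its rotation, and sets the pawn's SplineIndex to PedestrianSpline.
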(event EventBeginPlay
  (Utilities|FlowControl|Delay 2.5)
  (CallFunction|SpawnPedestrian)
  (Development|PrintString "swoosh"))

(fn ConstructionScript)

(fn SpawnPedestrian
  (bind _spline (Variables|Default|GetSpline))
  (bind _returnvalue (AI|SpawnAIFromClass "/Game/Blueprints/PC_Pedestrian.PC_Pedestrian_C" 0 (Spline|GetLocationatDistanceAlongSpline _spline 0.0 "World") (Spline|GetRotationatDistanceAlongSpline _spline 0.0 "World") false))
  (bind _aspc_pedestrian (Utilities|Casting|CastToPC_Pedestrian _returnvalue))
  (Variables|/Game/Blueprints/PC_Pedestrian.PC_Pedestrian_C|SetSplineIndex _aspc_pedestrian (Variables|Default|GetPedestrianSpline)))