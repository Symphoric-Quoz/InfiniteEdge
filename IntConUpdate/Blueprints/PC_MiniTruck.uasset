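; AI traffic mini truck that drives along a TrafficSpline picked by SplineIndex and destroys itself at the spline's end.
; Tick advances its distance by speed and axis value, setting position and rotation from the spline while keeping current height.
; Rear overlaps halt and release other trucks, and leaving the TrafficSpline triggers the next spawn.
; A truck still not clear after a three-second delay is destroyed and a replacement spawned.
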(event OnComponentEndOverlap(Rear)
  (params (OverlappedComponent :type Primitive%20Component%20Object%20Reference) (OtherActor :type Actor%20Object%20Reference) (OtherComp :type Primitive%20Component%20Object%20Reference) (OtherBodyIndex :type Integer))
  (Utilities|Casting|CastToTrafficSpline OtherActor
    (:then
      (Variables|Default|SetTrafficClear true)
      (Utilities|FlowControl|DoOnce false :!label _label
        (:Completed
          (Default|SpawnVehicle (Utilities|Array|Get(acopy) (Variables|Default|GetTrafficSplines) (Variables|Default|GetSplineIndex)))
          (Utilities|FlowControl|Delay 3.0)
          (goto _label Reset))))
    (:CastFailed
      (bind _aspc_mini_truck (Utilities|Casting|CastToPC_MiniTruck OtherActor))
      (if (Variables|PC_MiniTruck_C|GetCarStopped _aspc_mini_truck)
        (Variables|Default|SetCarStopped false)
        (Variables|PC_MiniTruck_C|SetCarSpeed _aspc_mini_truck 2e+02)))))

(event OnComponentBeginOverlap(Front)
  (params (OverlappedComponent :type Primitive%20Component%20Object%20Reference) (OtherActor :type Actor%20Object%20Reference) (OtherComp :type Primitive%20Component%20Object%20Reference) (OtherBodyIndex :type Integer) (bFromSweep :type Boolean) (SweepResult :type Hit%20Result%20Structure%20%28by%20ref%29)))

(event OnComponentEndOverlap(Front)
  (params (OverlappedComponent :type Primitive%20Component%20Object%20Reference) (OtherActor :type Actor%20Object%20Reference) (OtherComp :type Primitive%20Component%20Object%20Reference) (OtherBodyIndex :type Integer)))

(event OnComponentBeginOverlap(Rear)
  (params (OverlappedComponent :type Primitive%20Component%20Object%20Reference) (OtherActor :type Actor%20Object%20Reference) (OtherComp :type Primitive%20Component%20Object%20Reference) (OtherBodyIndex :type Integer) (bFromSweep :type Boolean) (SweepResult :type Hit%20Result%20Structure%20%28by%20ref%29))
  (bind _aspc_mini_truck (Utilities|Casting|CastToPC_MiniTruck OtherActor))
  (Variables|PC_MiniTruck_C|SetCarSpeed _aspc_mini_truck 0.0)
  (Variables|Default|SetCarStopped true))

(event OnComponentBeginOverlap(Sides)
  (params (OverlappedComponent :type Primitive%20Component%20Object%20Reference) (OtherActor :type Actor%20Object%20Reference) (OtherComp :type Primitive%20Component%20Object%20Reference) (OtherBodyIndex :type Integer) (bFromSweep :type Boolean) (SweepResult :type Hit%20Result%20Structure%20%28by%20ref%29)))

(event OnComponentEndOverlap(Sides)
  (params (OverlappedComponent :type Primitive%20Component%20Object%20Reference) (OtherActor :type Actor%20Object%20Reference) (OtherComp :type Primitive%20Component%20Object%20Reference) (OtherBodyIndex :type Integer)))

(event EventBeginPlay
  (bind _outactors (Actor|GetAllActorsOfClass "/Game/Blueprints/TrafficSpline.TrafficSpline_C"))
  (Variables|Default|SetTrafficSplines _outactors)
  (Variables|Default|SetVehicleSpline (Utilities|Array|Get(acopy) (Variables|Default|GetTrafficSplines) (Variables|Default|GetSplineIndex))))

(event EventTick
  (params (DeltaSeconds :type Float%20%28single-precision%29))
  (CallFunction|UpdateLocRot)
  (CallFunction|AddMovement)
  (Utilities|FlowControl|Delay 3.0)
  (if (not (Variables|Default|GetTrafficClear))
    (Actor|DestroyActor)
    (Default|SpawnVehicle (Utilities|Array|Get(acopy) (Variables|Default|GetTrafficSplines) (Variables|Default|GetSplineIndex)))))

(fn ConstructionScript)

(fn UpdateLocRot
  (bind _trafficsplines (Variables|Default|GetTrafficSplines))
  (bind _splineindex (Variables|Default|GetSplineIndex))
  (bind _distancealongspline (Variables|Default|GetDistanceAlongSpline))
  (bind _output (Utilities|Array|Get(acopy) _trafficsplines _splineindex))
  (bind _spline (Variables|/Game/Blueprints/TrafficSpline.TrafficSpline_C|GetSpline _output))
  (bind _returnvalue (Spline|GetLocationatDistanceAlongSpline _spline _distancealongspline "World"))
  (if (>= (Variables|Default|GetDistanceAlongSpline) (Spline|GetSplineLength (Variables|/Game/Blueprints/TrafficSpline.TrafficSpline_C|GetSpline (Variables|Default|GetVehicleSpline))))
    (Actor|DestroyActor)
    (else
      (Transformation|SetActorLocationAndRotation (Math|Vector|MakeVector (.x _returnvalue) (.y _returnvalue) (.z (Transformation|GetActorLocation))) (Spline|GetRotationatDistanceAlongSpline _spline (Variables|Default|GetDistanceAlongSpline) "World")))))

(fn AddMovement
  (bind _carspeed (Variables|Default|GetCarSpeed))
  (bind _axisvalue (Variables|Default|GetAxisValue))
  (bind _returnvalue (* _carspeed _axisvalue))
  (Variables|Default|SetCarAcceleration _returnvalue)
  (Variables|Default|SetDistanceAlongSpline (+ (Variables|Default|GetDistanceAlongSpline) (* _returnvalue (Utilities|Time|GetWorldDeltaSeconds)))))