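; Train actor that rides a TrainSpline chosen by SplineIndex, then destroys itself and asks that spline to spawn another train five seconds after BeginPlay.
; Each tick it snaps X, Y and rotation to the spline at DistanceAlongSpline, keeping its own Z, then advances that distance by speed, axis value and delta time.
; Reaching the spline's end also destroys it, while the stopped-or-blocked destroy branch is disabled by a constant condition.
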(event EventBeginPlay
  (bind _outactors (Actor|GetAllActorsOfClass "/Game/Blueprints/TrainSpline.TrainSpline_C"))
  (Variables|Default|SetTrainSplines _outactors)
  (Variables|Default|SetVehicleSpline (Utilities|Array|Get(acopy) (Variables|Default|GetTrainSplines) (Variables|Default|GetSplineIndex)))
  (Utilities|FlowControl|Delay 5.0)
  (Actor|DestroyActor)
  (Default|SpawnTrain (Utilities|Array|Get(acopy) (Variables|Default|GetTrainSplines) (Variables|Default|GetSplineIndex))))

(event EventTick
  (params (DeltaSeconds :type Float%20%28single-precision%29))
  (CallFunction|UpdateLocRot)
  (CallFunction|AddMovement)
  (if (not (and (not (Variables|Default|GetTrainStopped)) (Variables|Default|GetTrackClear)))
    (Utilities|FlowControl|Delay 2.0)
    (if (not true)
      (Actor|DestroyActor))))

(fn ConstructionScript)

(fn AddMovement
  (bind _trainspeed (Variables|Default|GetTrainSpeed))
  (bind _axisvalue (Variables|Default|GetAxisValue))
  (bind _returnvalue (* _trainspeed _axisvalue))
  (Variables|Default|SetTrainAcceleration _returnvalue)
  (Variables|Default|SetDistanceAlongSpline (+ (Variables|Default|GetDistanceAlongSpline) (* _returnvalue (Utilities|Time|GetWorldDeltaSeconds)))))

(fn UpdateLocRot
  (bind _splineindex (Variables|Default|GetSplineIndex))
  (bind _distancealongspline (Variables|Default|GetDistanceAlongSpline))
  (bind _trainsplines (Variables|Default|GetTrainSplines))
  (bind _output (Utilities|Array|Get(acopy) _trainsplines _splineindex))
  (bind _spline (Variables|/Game/Blueprints/TrainSpline.TrainSpline_C|GetSpline _output))
  (bind _returnvalue (Spline|GetLocationatDistanceAlongSpline _spline _distancealongspline "World"))
  (if (>= (Variables|Default|GetDistanceAlongSpline) (Spline|GetSplineLength (Variables|/Game/Blueprints/TrainSpline.TrainSpline_C|GetSpline (Variables|Default|GetVehicleSpline))))
    (Actor|DestroyActor)
    (else
      (Transformation|SetActorLocationAndRotation (Math|Vector|MakeVector (.x _returnvalue) (.y _returnvalue) (.z (Transformation|GetActorLocation))) (Spline|GetRotationatDistanceAlongSpline _spline (Variables|Default|GetDistanceAlongSpline) "World")))))