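; TrainSpline is a spline actor that spawns an AI train pawn at the start of its track.
; Its construction script stores the actor's own index within the list of all TrainSpline actors in the level.
; Shortly after BeginPlay, it spawns a PC_Train at the spline's first point and rotation.
; The spawned train receives that index as its SplineIndex, linking it to this spline.
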(event EventBeginPlay
  (Utilities|FlowControl|Delay 2.5)
  (CallFunction|SpawnTrain))

(fn ConstructionScript
  (bind _outactors (Actor|GetAllActorsOfClass "TrainSpline_C"))
  (Variables|Default|SetTrainSpline (Utilities|Array|FindItem _outactors self)))

(fn SpawnTrain
  (bind _spline (Variables|Default|GetSpline))
  (bind _returnvalue (AI|SpawnAIFromClass "/Game/Blueprints/PC_Train.PC_Train_C" 0 (Spline|GetLocationatDistanceAlongSpline _spline 0.0 "World") (Spline|GetRotationatDistanceAlongSpline _spline 0.0 "World") false))
  (bind _aspc_train (Utilities|Casting|CastToPC_Train _returnvalue))
  (Variables|/Game/Blueprints/PC_Train.PC_Train_C|SetSplineIndex _aspc_train (Variables|Default|GetTrainSpline)))