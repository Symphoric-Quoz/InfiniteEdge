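; BP_TrafficLight is a touch-controlled traffic light that stops PC_MiniTruck vehicles entering its Stopbox while not green.
; The overlap zeroes the truck's CarSpeed, sets CarStopped and stores it as the single VehicleStopped reference.
; Touching the Cube flip-flops LightIsGreen with debug prints; turning green restores the stored truck's speed but leaves CarStopped set.
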(event OnComponentBeginOverlap(Stopbox)
  (params (OverlappedComponent :type Primitive%20Component%20Object%20Reference) (OtherActor :type Actor%20Object%20Reference) (OtherComp :type Primitive%20Component%20Object%20Reference) (OtherBodyIndex :type Integer) (bFromSweep :type Boolean) (SweepResult :type Hit%20Result%20Structure%20%28by%20ref%29))
  (bind _aspc_mini_truck (Utilities|Casting|CastToPC_MiniTruck OtherActor))
  (if (not (Variables|Default|GetLightIsGreen))
    (Variables|/Game/Blueprints/PC_MiniTruck.PC_MiniTruck_C|SetCarSpeed _aspc_mini_truck 0.0)
    (Variables|Default|SetVehicleStopped _aspc_mini_truck)
    (Variables|/Game/Blueprints/PC_MiniTruck.PC_MiniTruck_C|SetCarStopped _aspc_mini_truck true)))

(event OnInputTouchBegin(Cube)
  (params (FingerIndex :type ETouchIndex%20Enum :default "Touch1") (TouchedComponent :type Primitive%20Component%20Object%20Reference))
  (Utilities|FlowControl|FlipFlop
    (:A
      (Variables|Default|SetLightIsGreen true)
      (Variables|/Game/Blueprints/PC_MiniTruck.PC_MiniTruck_C|SetCarSpeed (Variables|Default|GetVehicleStopped) 2e+02)
      (Development|PrintString "On"))
    (:B
      (Variables|Default|SetLightIsGreen false)
      (Development|PrintString "Off"))))

(fn ConstructionScript)