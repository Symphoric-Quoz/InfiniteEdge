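; PC_Pedestrian is a pedestrian actor that walks along one of the level's PedestrianSpline paths, selected by SplineIndex.
; Each tick it takes position and rotation from the spline while keeping its own Z, advances distance by PedSpeed times AxisValue, and destroys itself at the end.
; Capsule overlap with a spline flags WalkwayClear and spawns another pedestrian through a delay-reset DoOnce.
; Overlap with a stopped pedestrian clears its own PedStop flag.
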(event OnComponentBeginOverlap(CapsuleComponent)
  (params (OverlappedComponent :type Primitive%20Component%20Object%20Reference) (OtherActor :type Actor%20Object%20Reference) (OtherComp :type Primitive%20Component%20Object%20Reference) (OtherBodyIndex :type Integer) (bFromSweep :type Boolean) (SweepResult :type Hit%20Result%20Structure%20%28by%20ref%29))
  (Utilities|Casting|CastToPedestrianSpline OtherActor
    (:then
      (Variables|Default|SetWalkwayClear true)
      (Utilities|FlowControl|DoOnce false :!label _label
        (:Completed
          (Default|SpawnPedestrian (Utilities|Array|Get(acopy) (Variables|Default|GetPedestrianSplines) (Variables|Default|GetSplineIndex)))
          (Utilities|FlowControl|Delay 0.2)
          (Development|PrintString "that's a human person")
          (goto _label Reset))))
    (:CastFailed
      (bind _aspc_pedestrian (Utilities|Casting|CastToPC_Pedestrian OtherActor))
      (if (Variables|PC_Pedestrian_C|GetPedStop _aspc_pedestrian)
        (Variables|Default|SetPedStop false)))))

(event EventBeginPlay
  (bind _outactors (Actor|GetAllActorsOfClass "/Game/Blueprints/PedestrianSpline.PedestrianSpline_C"))
  (Variables|Default|SetPedestrianSplines _outactors)
  (Variables|Default|SetPedestrianSpline (Utilities|Array|Get(acopy) (Variables|Default|GetPedestrianSplines) (Variables|Default|GetSplineIndex))))

(event EventTick
  (params (DeltaSeconds :type Float%20%28single-precision%29))
  (CallFunction|UpdateLocRot)
  (CallFunction|AddMovement))

(fn ConstructionScript)

(fn UpdateLocRot
  (bind _pedestriansplines (Variables|Default|GetPedestrianSplines))
  (bind _splineindex (Variables|Default|GetSplineIndex))
  (bind _distancealongspline (Variables|Default|GetDistanceAlongSpline))
  (bind _output (Utilities|Array|Get(acopy) _pedestriansplines _splineindex))
  (bind _spline (Variables|/Game/Blueprints/PedestrianSpline.PedestrianSpline_C|GetSpline _output))
  (bind _returnvalue (Spline|GetLocationatDistanceAlongSpline _spline _distancealongspline "World"))
  (if (>= (Variables|Default|GetDistanceAlongSpline) (Spline|GetSplineLength (Variables|/Game/Blueprints/PedestrianSpline.PedestrianSpline_C|GetSpline (Variables|Default|GetPedestrianSpline))))
    (Actor|DestroyActor)
    (else
      (Transformation|SetActorLocationAndRotation (Math|Vector|MakeVector (.x _returnvalue) (.y _returnvalue) (.z (Transformation|GetActorLocation))) (Spline|GetRotationatDistanceAlongSpline _spline (Variables|Default|GetDistanceAlongSpline) "World")))))

(fn AddMovement
  (bind _pedspeed (Variables|Default|GetPedSpeed))
  (bind _axisvalue (Variables|Default|GetAxisValue))
  (bind _returnvalue (* _pedspeed _axisvalue))
  (Variables|Default|SetPedAcceleration _returnvalue)
  (Variables|Default|SetDistanceAlongSpline (+ (Variables|Default|GetDistanceAlongSpline) (* _returnvalue (Utilities|Time|GetWorldDeltaSeconds)))))