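; PC_MiniTruck is a traffic vehicle that drives along an indexed TrafficSpline each Tick and destroys itself at the end.
; Front and rear triggers track traffic clearance, halt and release queued trucks, and turn cross-lane contact into a crash that tints, stops and shoves the trucks.
; Box overlaps with a spline add player score.
; Spline completion adds TimeScore to a newly created HUD widget, while waiting trucks without clearance are destroyed.
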(event OnComponentEndOverlap(Rear)
  (params (OverlappedComponent :type Primitive%20Component%20Object%20Reference) (OtherActor :type Actor%20Object%20Reference) (OtherComp :type Primitive%20Component%20Object%20Reference) (OtherBodyIndex :type Integer))
  (Utilities|Casting|CastToTrafficSpline OtherActor
    (:then
      (Variables|Default|SetTrafficClear true))
    (:CastFailed
      (bind _aspc_mini_truck (Utilities|Casting|CastToPC_MiniTruck OtherActor))
      (if (Variables|PC_MiniTruck_C|GetCarStopped _aspc_mini_truck)
        (Variables|Default|SetCarStopped false)
        (Variables|PC_MiniTruck_C|SetCarSpeed _aspc_mini_truck 2e+02)))))

(event OnComponentBeginOverlap(Front)
  (params (OverlappedComponent :type Primitive%20Component%20Object%20Reference) (OtherActor :type Actor%20Object%20Reference) (OtherComp :type Primitive%20Component%20Object%20Reference) (OtherBodyIndex :type Integer) (bFromSweep :type Boolean) (SweepResult :type Hit%20Result%20Structure%20%28by%20ref%29))
  (bind _aspc_mini_truck (Utilities|Casting|CastToPC_MiniTruck OtherActor))
  (if (and (!= (Variables|Default|GetSplineIndex) (Variables|PC_MiniTruck_C|GetSplineIndex _aspc_mini_truck)) (Variables|PC_MiniTruck_C|GetTrafficClear _aspc_mini_truck))
    (Sprite|SetSpriteColor (Variables|/Script/Paper2D.PaperCharacter|GetSprite _aspc_mini_truck) "(R=0.566323,G=0.000000,B=1.000000,A=1.000000)")
    (Utilities|Array|AddUnique (Variables|Default|GetHitVehicles) _aspc_mini_truck)
    (for _array_element (Variables|Default|GetHitVehicles)
      (Variables|PC_MiniTruck_C|SetCarSpeed _array_element 0.0)
      (Variables|Default|SetInAccident true))
    (Variables|Default|SetVehicleOffset (* (- (Transformation|GetActorLocation OtherActor) (Transformation|GetActorLocation)) 25.0))
    (for _array_element_2 (Variables|Default|GetHitVehicles)
      (Transformation|AddActorWorldOffset _array_element_2 (Variables|Default|GetVehicleOffset))
      (Transformation|SetActorRotation _array_element_2 (Math|Rotator|MakeRotator (.roll (Transformation|GetActorRotation _array_element_2)) (.pitch (Transformation|GetActorRotation _array_element_2)) (- (.yaw (Transformation|GetActorRotation _array_element_2)) 2e+01))))
    (Utilities|FlowControl|Delay 0.025)
    (Variables|Default|SetVehicleOffset "0, 0, 0")
    (Utilities|FlowControl|Delay 0.125)
    (for _array_element_3 (Variables|Default|GetHitVehicles)
      (Collision|SetCollisionEnabled (Variables|PC_MiniTruck_C|GetFront _array_element_3) "NoCollision"))))

(event OnComponentEndOverlap(Front)
  (params (OverlappedComponent :type Primitive%20Component%20Object%20Reference) (OtherActor :type Actor%20Object%20Reference) (OtherComp :type Primitive%20Component%20Object%20Reference) (OtherBodyIndex :type Integer))
  (Utilities|Casting|CastToTrafficSpline OtherActor
    (:then
      (Variables|Default|SetTrafficClear true))
    (:CastFailed
      (bind _aspc_mini_truck (Utilities|Casting|CastToPC_MiniTruck OtherActor))
      (if (Variables|PC_MiniTruck_C|GetCarStopped _aspc_mini_truck)
        (Variables|Default|SetCarStopped false)
        (Variables|PC_MiniTruck_C|SetCarSpeed _aspc_mini_truck 2e+02)))))

(event OnInputTouchBegin(Sides)
  (params (FingerIndex :type ETouchIndex%20Enum :default "Touch1") (TouchedComponent :type Primitive%20Component%20Object%20Reference))
  (Variables|Default|SetCarStopped false)
  (Development|PrintString "Go"))

(event OnComponentBeginOverlap(Rear)
  (params (OverlappedComponent :type Primitive%20Component%20Object%20Reference) (OtherActor :type Actor%20Object%20Reference) (OtherComp :type Primitive%20Component%20Object%20Reference) (OtherBodyIndex :type Integer) (bFromSweep :type Boolean) (SweepResult :type Hit%20Result%20Structure%20%28by%20ref%29))
  (bind _aspc_mini_truck (Utilities|Casting|CastToPC_MiniTruck OtherActor))
  (Variables|PC_MiniTruck_C|SetCarSpeed _aspc_mini_truck 0.0)
  (Variables|Default|SetCarStopped true)
  (Variables|Default|SetInWaiting true))

(event OnComponentBeginOverlap(Sides)
  (params (OverlappedComponent :type Primitive%20Component%20Object%20Reference) (OtherActor :type Actor%20Object%20Reference) (OtherComp :type Primitive%20Component%20Object%20Reference) (OtherBodyIndex :type Integer) (bFromSweep :type Boolean) (SweepResult :type Hit%20Result%20Structure%20%28by%20ref%29))
  (if (Variables|Default|GetInAccident)
    _))

(event OnComponentEndOverlap(Sides)
  (params (OverlappedComponent :type Primitive%20Component%20Object%20Reference) (OtherActor :type Actor%20Object%20Reference) (OtherComp :type Primitive%20Component%20Object%20Reference) (OtherBodyIndex :type Integer)))

(event OnComponentBeginOverlap(Box)
  (params (OverlappedComponent :type Primitive%20Component%20Object%20Reference) (OtherActor :type Actor%20Object%20Reference) (OtherComp :type Primitive%20Component%20Object%20Reference) (OtherBodyIndex :type Integer) (bFromSweep :type Boolean) (SweepResult :type Hit%20Result%20Structure%20%28by%20ref%29))
  (Utilities|Casting|CastToTrafficSpline OtherActor)
  (bind _asplayer_character (Utilities|Casting|CastToPlayerCharacter (Game|GetPlayerCharacter 0)))
  (bind _output_get (Variables|/Game/Blueprints/PlayerCharacter.PlayerCharacter_C|SetScore _asplayer_character (+ (Variables|/Game/Blueprints/PlayerCharacter.PlayerCharacter_C|GetScore _asplayer_character) 1e+01)))
  (Development|PrintString "POINT REGISTERED")
  (Development|PrintString (Utilities|String|ToString(Float) _output_get)))

(event EventBeginPlay
  (bind _outactors (Actor|GetAllActorsOfClass "/Game/Blueprints/TrafficSpline.TrafficSpline_C"))
  (Variables|Default|SetTrafficSplines _outactors)
  (Variables|Default|SetVehicleSpline (Utilities|Array|Get(acopy) (Variables|Default|GetTrafficSplines) (Variables|Default|GetSplineIndex)))
  (Development|PrintString "linked to line"))

(event EventTick
  (params (DeltaSeconds :type Float%20%28single-precision%29))
  (CallFunction|UpdateLocRot)
  (CallFunction|AddMovement)
  (Utilities|FlowControl|Delay 3.0)
  (if (Variables|Default|GetInWaiting)
    (Development|PrintString "is waiting")
    (if (not (Variables|Default|GetTrafficClear))
      (Actor|DestroyActor)
      (Utilities|FlowControl|Delay (Math|Random|RandomFloatinRange 3.0 15.0)))))

(fn ConstructionScript)

(fn UpdateLocRot
  (bind _trafficsplines (Variables|Default|GetTrafficSplines))
  (bind _splineindex (Variables|Default|GetSplineIndex))
  (bind _distancealongspline (Variables|Default|GetDistanceAlongSpline))
  (bind _output (Utilities|Array|Get(acopy) _trafficsplines _splineindex))
  (bind _spline (Variables|/Game/Blueprints/TrafficSpline.TrafficSpline_C|GetSpline _output))
  (bind _returnvalue (Spline|GetLocationatDistanceAlongSpline _spline _distancealongspline "World"))
  (if (>= (Variables|Default|GetDistanceAlongSpline) (Spline|GetSplineLength (Variables|/Game/Blueprints/TrafficSpline.TrafficSpline_C|GetSpline (Variables|Default|GetVehicleSpline))))
    (Actor|DestroyActor)
    (Development|PrintString "ascend")
    (bind _returnvalue_2 (UserInterface|CreateWidget "/Game/Blueprints/UI/DAD_Functions/Wid_PlayerHUD.Wid_PlayerHUD_C"))
    (bind _output_get (Variables|Default|SetScore (+ (Variables|/Game/Blueprints/UI/DAD_Functions/Wid_PlayerHUD.Wid_PlayerHUD_C|GetTimeScore _returnvalue_2) 1000)))
    (Development|PrintString (Utilities|String|ToString(Integer) _output_get))
    (Variables|/Game/Blueprints/UI/DAD_Functions/Wid_PlayerHUD.Wid_PlayerHUD_C|SetTimeScore _returnvalue_2 _output_get)
    (else
      (Transformation|SetActorLocationAndRotation (Math|Vector|MakeVector (.x _returnvalue) (.y _returnvalue) (.z (Transformation|GetActorLocation))) (Spline|GetRotationatDistanceAlongSpline _spline (Variables|Default|GetDistanceAlongSpline) "World")))))

(fn AddMovement
  (bind _carspeed (Variables|Default|GetCarSpeed))
  (bind _axisvalue (Variables|Default|GetAxisValue))
  (bind _returnvalue (* _carspeed _axisvalue))
  (Variables|Default|SetCarAcceleration _returnvalue)
  (Variables|Default|SetDistanceAlongSpline (+ (Variables|Default|GetDistanceAlongSpline) (* _returnvalue (Utilities|Time|GetWorldDeltaSeconds)))))